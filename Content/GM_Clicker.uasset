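; Game mode for a clicker game that creates the main UI widget at start and applies coin and level changes to the player state.
; It caches PS_Player_Data and rebinds handlers to its Upgrade and GetCoin dispatchers every Tick.
; GetCoin adds a fixed amount of coins, while Upgrade spends coins at a cost proportional to Level to raise it by one, if affordable.
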(event Custom|CustomEvent
  (Variables|/Game/PS_Player_Data.PS_Player_Data_C|SetCoin (Variables|Default|GetAs%20PS%20Player%20Data) (+ (Variables|/Game/PS_Player_Data.PS_Player_Data_C|GetCoin (Variables|Default|GetAs%20PS%20Player%20Data)) 10)))

(event Custom|CustomEvent_0
  (if (>= (Variables|/Game/PS_Player_Data.PS_Player_Data_C|GetCoin (Variables|Default|GetAs%20PS%20Player%20Data)) (* (Variables|/Game/PS_Player_Data.PS_Player_Data_C|GetLevel (Variables|Default|GetAs%20PS%20Player%20Data)) 100))
    (Utilities|FlowControl|Sequence
      (:then_0
        (Variables|/Game/PS_Player_Data.PS_Player_Data_C|SetCoin (Variables|Default|GetAs%20PS%20Player%20Data) (- (Variables|/Game/PS_Player_Data.PS_Player_Data_C|GetCoin (Variables|Default|GetAs%20PS%20Player%20Data)) (* (Variables|/Game/PS_Player_Data.PS_Player_Data_C|GetLevel (Variables|Default|GetAs%20PS%20Player%20Data)) 100))))
      (:then_1
        (Variables|/Game/PS_Player_Data.PS_Player_Data_C|SetLevel (Variables|Default|GetAs%20PS%20Player%20Data) (+ (Variables|/Game/PS_Player_Data.PS_Player_Data_C|GetLevel (Variables|Default|GetAs%20PS%20Player%20Data)) 1))))))

(event EventBeginPlay
  (Utilities|FlowControl|Sequence
    (:then_0
      (bind _returnvalue (UserInterface|CreateWidget "/Game/WB_Main_UI.WB_Main_UI_C"))
      (UserInterface|Viewport|AddtoViewport _returnvalue 0))
    (:then_1
      (bind _asps_player_data (Utilities|Casting|CastToPS_Player_Data (Game|GetPlayerState 0)))
      (Variables|Default|SetAs%20PS%20Player%20Data _asps_player_data))))

(event EventTick
  (params (DeltaSeconds :type Float%20%28single-precision%29))
  (Utilities|FlowControl|Sequence
    (:then_0
      (EventDispatchers|BindEventtoUpgrade (delegate Custom|CustomEvent_0)))
    (:then_1
      (EventDispatchers|BindEventtoGetCoin (delegate Custom|CustomEvent)))))

(fn ConstructionScript)